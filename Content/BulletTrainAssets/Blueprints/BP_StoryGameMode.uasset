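; Story-mode game mode that takes the player from a story selection screen to a chosen story.
; On BeginPlay it caches BP_GameManager from the game instance, shows BP_StorySelect and pre-creates BP_Story.
; SeeStory stores the chapter and stage indices, swaps the widgets and initializes BP_Story with the matching entry from the manager's StoryData.
; MoveGame is an empty stub.
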(event `self.ReceiveBeginPlay`
  (bind _asbp_game_manager (cast `/Game/BulletTrainAssets/Blueprints/BP_GameManager` (`GameplayStatics.GetGameInstance`)))
  (set `self.GameManager` _asbp_game_manager)
  (bind _returnvalue (`|CreateWidget` "/Game/BulletTrainAssets/Blueprints/HUD/Story/BP_StorySelect.BP_StorySelect_C"))
  (bind _output_get (set `self.StorySelectUI` _returnvalue))
  (`UserWidget.AddToViewport` _output_get 0)
  (bind _returnvalue_2 (`|CreateWidget` "/Game/BulletTrainAssets/Blueprints/HUD/Story/BP_Story.BP_Story_C"))
  (set `self.StoryUI` _returnvalue_2))

(event `SeeStory`
  (params (Chapter :type Integer) (Stage :type Integer))
  (bind _storyui (`self.StoryUI`))
  (bind _output_get (set `self.ChapterIndex` Chapter))
  (bind _output_get_2 (set `self.StageIndex` Stage))
  (`Widget.RemoveFromParent` (`self.StorySelectUI`))
  (`UserWidget.AddToViewport` _storyui 0)
  (bind _asbp_story (cast `/Game/BulletTrainAssets/Blueprints/HUD/Story/BP_Story` _storyui))
  (`/Game/BulletTrainAssets/Blueprints/HUD/Story/BP_Story.InitStory` _asbp_story (`|GetArrayItem` (`.StoryStageDatas_4_5F8B9B214B4314A79CF255B8A2494AE1` (break `/Game/BulletTrainAssets/Structure/StoryData` (`|GetArrayItem` (`/Game/BulletTrainAssets/Blueprints/BP_GameManager.StoryData` (`self.GameManager`)) _output_get))) _output_get_2)))

(event `MoveGame`)

(fn `UserConstructionScript`)