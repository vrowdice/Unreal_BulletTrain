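; Alliance actor that penalizes the player's trust when it is hit by a bullet.
; BeginPlay caches the BP_GameManager game instance and the BP_MainGameMode game mode.
; HitByBullet plays a hit sound at the world origin, scaled by the manager's effect volume, then passes the damage to the game mode's DecreaseTrust.
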(event `self.ReceiveBeginPlay`
  (bind _asbp_game_data_manager (cast `/Game/BulletTrainAssets/Blueprints/BP_GameManager` (`GameplayStatics.GetGameInstance`)))
  (set `self.GameDataManager` _asbp_game_data_manager)
  (bind _asbp_main_game_mode (cast `/Game/BulletTrainAssets/Blueprints/BP_MainGameMode` (`GameplayStatics.GetGameMode`)))
  (set `self.GameMode` _asbp_main_game_mode))

(fn `HitByBullet`
  (params (Damage :type "Float (double-precision)"))
  (`GameplayStatics.PlaySoundAtLocation` "/Game/BulletTrainAssets/Sound/AlienceHit/AlienceHit2.AlienceHit2" (0.0 0.0 0.0) (struct) (`/Game/BulletTrainAssets/Blueprints/BP_GameManager.EffectSoundVolum` (`self.GameDataManager`)) 1.0 0.0 null null null null)
  (`/Game/BulletTrainAssets/Blueprints/BP_MainGameMode.DecreaseTrust` (`self.GameMode`) Damage))