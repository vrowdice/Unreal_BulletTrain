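; Game mode for the title screen, managing the title and weapon setting menus with a moving camera.
; On BeginPlay it spawns BP_Camera as the view target, shows the mouse cursor and creates both widgets, displaying the title one.
; Switching menus swaps the widgets and smoothly moves the camera between two stored transforms.
; Story select opens the map named in the BP_GameManager game instance.
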(event `self.ReceiveBeginPlay`
  (bind _returnvalue (`GameplayStatics.GetPlayerController` 0))
  (bind _returnvalue_2 (`|SpawnActorFromClass` "/Game/BulletTrainAssets/Blueprints/Character/BP_Camera.BP_Camera_C" (`self.TitleCameraTrans`) "Undefined" "OverrideRootScale" null null))
  (bind _asbp_camera (cast `/Game/BulletTrainAssets/Blueprints/Character/BP_Camera` _returnvalue_2))
  (bind _output_get (set `self.Camera` _asbp_camera))
  (`PlayerController.SetViewTargetWithBlend` _returnvalue _output_get 0.0 "VTBlend_Linear" 0.0 false)
  (set `PlayerController.bShowMouseCursor` true _returnvalue)
  (bind _returnvalue_3 (`|CreateWidget` "/Game/BulletTrainAssets/Blueprints/HUD/Title/BP_Tiltle.BP_Tiltle_C"))
  (bind _output_get_2 (set `self.TitleUI` _returnvalue_3))
  (`UserWidget.AddToViewport` _output_get_2 0)
  (bind _returnvalue_4 (`|CreateWidget` "/Game/BulletTrainAssets/Blueprints/HUD/Title/BP_WeaponSetting.BP_WeaponSetting_C"))
  (set `self.WeaponSettingUI` _returnvalue_4))

(event `OpenStorySelect`
  (bind _asbp_game_manager (cast `/Game/BulletTrainAssets/Blueprints/BP_GameManager` (`GameplayStatics.GetGameInstance`)))
  (`GameplayStatics.OpenLevel` (`/Game/BulletTrainAssets/Blueprints/BP_GameManager.StoryMapName` _asbp_game_manager)))

(event `OpenWeaponSetting`
  (`Widget.RemoveFromParent` (`self.TitleUI`))
  (`UserWidget.AddToViewport` (`self.WeaponSettingUI`) 0)
  (`/Game/BulletTrainAssets/Blueprints/Character/BP_Camera.MoveSmoth` (`self.Camera`) (`self.TitleCameraTrans`) (`self.WeaponSettingCameraVecTrans`)))

(event `BackTitle`
  (`Widget.RemoveFromParent` (`self.WeaponSettingUI`))
  (`UserWidget.AddToViewport` (`self.TitleUI`) 0)
  (`/Game/BulletTrainAssets/Blueprints/Character/BP_Camera.MoveSmoth` (`self.Camera`) (`self.WeaponSettingCameraVecTrans`) (`self.TitleCameraTrans`)))

(fn `UserConstructionScript`)