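; BP_EnemyManager spawns enemy ships on timed intervals, driven by enemy and spawn settings in the game data manager.
; A looping timer adds the base interval to each enemy type's accumulated time, spawning it and resetting once its spawn time is reached, then writes the entry back.
; Spawns use a fixed X and random Y/Z within configured bounds, add a BP_EnemyShip component carrying that type's stats and weapon data, and get rotated.
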(event `self.ReceiveBeginPlay`
  (bind _asbp_game_data_manager (cast `/Game/BulletTrainAssets/Blueprints/Manager/BP_GameDataManager` (`GameplayStatics.GetGameInstance`)))
  (bind _output_get (set `self.GameDataManager` _asbp_game_data_manager))
  (bind _asbp_main_game_mode (cast `/Game/BulletTrainAssets/Blueprints/BP_MainGameMode` (`GameplayStatics.GetGameMode`)))
  (set `self.GameMode` _asbp_main_game_mode)
  (`KismetSystemLibrary.K2_SetTimer` null "Timer" (`/Game/BulletTrainAssets/Blueprints/Manager/BP_GameDataManager.TimerIntervalBase` _output_get) true))

(fn `SpawnRandomSpace`
  (params (EnemyData :type "/Game/BulletTrainAssets/Blueprints/Structure/Enemy/EnemyData Structure"))
  (bind (_actor _name _hp _iscloserangeshoot _size _speed _spawntime _delaystartspawntime _calspawntime _weapondata) (break `/Game/BulletTrainAssets/Blueprints/Structure/Enemy/EnemyData` EnemyData))
  (bind (_difficultymultiplier _spawnpositionx _destroypositionx _targetspawnpoint _weaponspawnpoint _spawnspacesqarepoint1 _spawnspacesqarepoint2) (break `/Game/BulletTrainAssets/Blueprints/Structure/SpawnSettingData` (`/Game/BulletTrainAssets/Blueprints/Manager/BP_GameDataManager.SpawnSettingData` (`self.GameDataManager`))))
  (bind _returnvalue (`|SpawnActorFromClass` _actor (`KismetMathLibrary.Conv_VectorToTransform` (`KismetMathLibrary.MakeVector` _spawnpositionx (`KismetMathLibrary.RandomFloatInRange` (.y _spawnspacesqarepoint1) (.y _spawnspacesqarepoint2)) (`KismetMathLibrary.RandomFloatInRange` (.z _spawnspacesqarepoint1) (.z _spawnspacesqarepoint2)))) "Undefined" "OverrideRootScale" null null))
  (`|AddComponentByClass` _returnvalue "/Game/BulletTrainAssets/Blueprints/Enemey/BP_EnemyShip.BP_EnemyShip_C" (`self.GameDataManager`) (`self.GameMode`) _speed _destroypositionx _size _hp _iscloserangeshoot _weapondata)
  (`self.K2_SetActorRotation` _returnvalue (struct :`Yaw` 180.0) false))

(fn `Timer`
  (bind _gamedatamanager (`self.GameDataManager`))
  (bind _enemydata (`/Game/BulletTrainAssets/Blueprints/Manager/BP_GameDataManager.EnemyData` _gamedatamanager))
  (for (_array_element _array_index) _enemydata
    (bind _structout (setmembers `/Game/BulletTrainAssets/Blueprints/Structure/Enemy/EnemyData` :`StructRef` _array_element :`CalSpawnTime` (+ (`.CalSpawnTime_4_E9D18BB743F74E3F53DFBCA8823733BD` (break `/Game/BulletTrainAssets/Blueprints/Structure/Enemy/EnemyData` _array_element)) (`/Game/BulletTrainAssets/Blueprints/Manager/BP_GameDataManager.TimerIntervalBase` _gamedatamanager))))
    (bind (_actor _name _hp _iscloserangeshoot _size _speed _spawntime _delaystartspawntime _calspawntime) (break `/Game/BulletTrainAssets/Blueprints/Structure/Enemy/EnemyData` _structout))
    (if (<= _spawntime _calspawntime)
      (bind _structout_2 (setmembers `/Game/BulletTrainAssets/Blueprints/Structure/Enemy/EnemyData` :`StructRef` _structout :`CalSpawnTime` 0.0))
      (`self.SpawnRandomSpace` _structout_2)
      (`KismetArrayLibrary.Array_Set` _enemydata _array_index _structout_2)
      (else
        (`KismetArrayLibrary.Array_Set` _enemydata _array_index _structout)))))

(fn `UserConstructionScript`)