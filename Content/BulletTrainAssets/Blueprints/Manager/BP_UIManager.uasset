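; BP_UIManager is a UI manager Blueprint that prepares score text and a fading score-gain popup value.
; GetScore adds each gain to a running sum, stores it and the BP_MainGameMode total as strings, and resets the alpha to full.
; A looping timer runs GetScoreOver, easing the alpha toward zero, then clears itself and the sum.
; Because alpha is set before its check, the non-accumulating branch never runs.
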(fn `GetScore`
  (params (Score :type Integer))
  (bind _asbp_main_game_mode (cast `/Game/BulletTrainAssets/Blueprints/BP_MainGameMode` (`GameplayStatics.GetGameMode`)))
  (bind _output_get (set `self.GetScoreAlpha` 1.0))
  (if (> _output_get 0.0)
    (bind _output_get_2 (set `self.GetScoreTmp` (+ (`self.GetScoreTmp`) Score)))
    (set `self.GetScoreStr` (`KismetStringLibrary.Conv_IntToString` _output_get_2))
    (else
      (set `self.GetScoreStr` (`KismetStringLibrary.Conv_IntToString` Score))))
  (set `self.ScoreStr` (`KismetStringLibrary.Conv_IntToString` (`/Game/BulletTrainAssets/Blueprints/BP_MainGameMode.Score` _asbp_main_game_mode)))
  (`KismetSystemLibrary.K2_SetTimer` null "GetScoreOver" (`self.AlphaChangeTime`) true))

(fn `GetScoreOver`
  (bind _output_get (set `self.GetScoreAlpha` (`KismetMathLibrary.FInterpTo_Constant` (`self.GetScoreAlpha`) 0.0 (`GameplayStatics.GetWorldDeltaSeconds`) 1.0)))
  (if (<= _output_get 0.0)
    (`KismetSystemLibrary.K2_ClearTimer` null "GetScoreOver")
    (set `self.GetScoreTmp` 0)))

(fn `UserConstructionScript`)