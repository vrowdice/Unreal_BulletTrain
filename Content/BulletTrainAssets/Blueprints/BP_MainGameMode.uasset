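; BP_MainGameMode is the game mode that tracks score and trust to decide when the game ends in a win or loss.
; On BeginPlay it spawns the enemy manager, UI manager and space station target, and fills Trust to its maximum.
; Reaching the goal score or depleting trust triggers GameOver, which sets the win flag, pauses after a short delay and shows the game-over UI with the cursor.
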(event `self.ReceiveBeginPlay`
  (bind _returnvalue (`KismetMathLibrary.Conv_VectorToTransform` (`KismetMathLibrary.Vector_Zero`)))
  (bind _returnvalue_2 (`|SpawnActorFromClass` "/Game/BulletTrainAssets/Blueprints/Manager/BP_EnemyManager.BP_EnemyManager_C" _returnvalue "Undefined" "OverrideRootScale" null null))
  (set `self.EnemyManager` _returnvalue_2)
  (bind _returnvalue_3 (`|SpawnActorFromClass` "/Game/BulletTrainAssets/Blueprints/Manager/BP_UIManager.BP_UIManager_C" _returnvalue "Undefined" "OverrideRootScale" null null))
  (set `self.UIManager` _returnvalue_3)
  (set `self.Trust` (`self.MaxTrust`))
  (bind _returnvalue_4 (`|SpawnActorFromClass` "/Game/BulletTrainAssets/Blueprints/Alliance/BP_SpaceStationTarget.BP_SpaceStationTarget_C" (`KismetMathLibrary.Conv_VectorToTransform` (`.TargetSpawnPoint_59_67016D44407ECB4EE5BC0D9A20C60229` (break `/Game/BulletTrainAssets/Blueprints/Structure/SpawnSettingData` (`self.SpawnSetting`)))) "Undefined" "OverrideRootScale" null null))
  (set `self.StationTarget` _returnvalue_4))

(event `GameOver`
  (if (<= (`self.Trust`) 0.0)
    (set `self.IsWin` false)
    (else
      (set `self.IsWin` true)))
  (`KismetSystemLibrary.Delay` 1.0)
  (`GameplayStatics.SetGamePaused` true)
  (set `PlayerController.bShowMouseCursor` true (`GameplayStatics.GetPlayerController` 0))
  (bind _returnvalue (`|CreateWidget` "/Game/BulletTrainAssets/Blueprints/UI/GameOverUI.GameOverUI_C"))
  (`UserWidget.AddToViewport` _returnvalue 0))

(fn `DecreaseTrust`
  (params (DecreaseTrust :type "Float (double-precision)"))
  (bind _output_get (set `self.Trust` (- (`self.Trust`) DecreaseTrust)))
  (if (<= _output_get 0.0)
    (`self.GameOver`)))

(fn `GetScore`
  (params (ScoreIn :type Integer))
  (returns (ScoreOut :type Integer))
  (bind _output_get (set `self.Score` (+ ScoreIn (`self.Score`))))
  (if (<= (`self.GoalScore`) (`self.Score`))
    (`self.GameOver`))
  (`/Game/BulletTrainAssets/Blueprints/Manager/BP_UIManager.GetScore` (`self.UIManager`) ScoreIn)
  (return _output_get))

(fn `UserConstructionScript`)