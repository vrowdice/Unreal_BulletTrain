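; Enemy ship that warps in, flies forward firing at the station target, and warps out past a map X limit.
; Tick moves it and uses Delay to pace either close-range bullets or homing missiles, depending on flags.
; HitByBullet subtracts HP and awards score, flagging destruction at zero.
; A destroyed ship decelerates amid small explosions, then explodes and is removed once stopped.
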(event `self.ReceiveBeginPlay`
  (bind _gamedatamanager (`self.GameDataManager`))
  (bind _location (.location (`Actor.GetTransform` (`self.GetOwner`))))
  (set `self.Hp` (`self.MaxHp`))
  (set `self.Speed` (`self.MaxSpeed`))
  (`GameplayStatics.PlaySoundAtLocation` (`.WarpIn_13_D40F47C64921382E46F48E8B3EB9F648` (break `/Game/BulletTrainAssets/Blueprints/Structure/CommonEffectSoundData` (`/Game/BulletTrainAssets/Blueprints/Manager/BP_GameDataManager.EffectSoundData` _gamedatamanager))) _location (struct) (`/Game/BulletTrainAssets/Blueprints/Manager/BP_GameDataManager.EffectSoundVolum` _gamedatamanager) 1.0 0.0 null null null null)
  (`GameplayStatics.SpawnEmitterAtLocation` "/Game/BulletTrainAssets/Particles/P_Warp.P_Warp" _location (struct) (5.0 5.0 5.0)))

(event `self.ReceiveTick`
  (params (DeltaSeconds :type "Float (single-precision)"))
  (bind _returnvalue (`self.GetOwner`))
  (bind (_actor _firerate _damage) (break `/Game/BulletTrainAssets/Blueprints/Structure/Weapon/EnemyWeaponData` (`self.WeaponData`)))
  (bind _returnvalue_2 (`Actor.GetTransform` (`self.GetOwner`)))
  (bind _returnvalue_3 (`Actor.K2_GetActorLocation` _returnvalue))
  (bind _stationtarget (`/Game/BulletTrainAssets/Blueprints/BP_MainGameMode.StationTarget` (`self.GameMode`)))
  (bind (_finaldestroymul _interpspeedmul _destroyemitspawninterval) (break `/Game/BulletTrainAssets/Blueprints/Structure/Enemy/EnemySettingData` (`/Game/BulletTrainAssets/Blueprints/Manager/BP_GameDataManager.EnemySetting` (`self.GameDataManager`))))
  (bind (_backgroundsound _smallexplosion _bigexplosion) (break `/Game/BulletTrainAssets/Blueprints/Structure/CommonEffectSoundData` (`/Game/BulletTrainAssets/Blueprints/Manager/BP_GameDataManager.EffectSoundData` (`self.GameDataManager`))))
  ;[1 1 1] Move
  (`Actor.K2_SetActorLocation` _returnvalue (+ (`Actor.K2_GetActorLocation` _returnvalue) (* (`Actor.GetActorForwardVector` _returnvalue) (`self.Speed`) DeltaSeconds)) true false)
  (if (<= (`self.Speed`) 0.0)
    ;[1 1 1] Stop Destroy
    (`GameplayStatics.PlaySoundAtLocation` _bigexplosion _returnvalue_3 (struct) (`/Game/BulletTrainAssets/Blueprints/Manager/BP_GameDataManager.EffectSoundVolum` (`self.GameDataManager`)) 1.0 0.0 null null null null)
    ;[1 1 1] Out of Map Destroy
    (`GameplayStatics.SpawnEmitterAtLocation` "/Game/BulletTrainAssets/Particles/P_Explosion.P_Explosion" _returnvalue_3 (struct) (`KismetMathLibrary.Conv_DoubleToVector` (`self.Size`)))
    (`/Engine/EditorBlueprintResources/StandardMacros.IsValid` _returnvalue :!label _label
      (:`Is Valid`
        (`Actor.K2_DestroyActor` _returnvalue)))
    (elif (<= (.x _returnvalue_3) (`self.DestroyXPos`))
      (`GameplayStatics.SpawnEmitterAtLocation` "/Game/BulletTrainAssets/Particles/P_Warp.P_Warp" (.location (`Actor.GetTransform` _returnvalue)) (struct) (5.0 5.0 5.0))
      (goto _label)
      (elif (`self.IsDestroy`)
        ;[1 1 1] No HP than Slow Down Speed
        (set `self.IsCloseRangeShoot` false)
        (set `self.Speed` (`KismetMathLibrary.FInterpTo_Constant` (`self.Speed`) 0.0 DeltaSeconds (* _interpspeedmul (`self.MaxSpeed`))))
        (`KismetSystemLibrary.Delay` _destroyemitspawninterval)
        (`GameplayStatics.PlaySoundAtLocation` _smallexplosion _returnvalue_3 (struct) (`/Game/BulletTrainAssets/Blueprints/Manager/BP_GameDataManager.EffectSoundVolum` (`self.GameDataManager`)) 1.0 0.0 null null null null)
        (`GameplayStatics.SpawnEmitterAtLocation` "/Game/StarterContent/Particles/P_Explosion.P_Explosion" _returnvalue_3 (struct) (* (`self.Size`) (`self.SmallExplosionMul`)))
        (elif (`self.IsCloseRangeShoot`)
          ;[1 1 1] Spawn Enemy Bullet
          (if (`self.IsCloseRangeShootStart`)
            (`KismetSystemLibrary.Delay` _firerate)
            (`|SpawnActorFromClass` "/Game/BulletTrainAssets/Blueprints/Weapon/EnemyBullet/BP_EnemyBullet.BP_EnemyBullet_C" _returnvalue_2 "Undefined" "OverrideRootScale" null _stationtarget _damage null))
          (else
            ;[1 1 1] Spawn Missile
            (`KismetSystemLibrary.Delay` _firerate)
            (`|SpawnActorFromClass` "/Game/BulletTrainAssets/Blueprints/Weapon/EnemyBullet/BP_EnemyMissile.BP_EnemyMissile_C" _returnvalue_2 "Undefined" "OverrideRootScale" null (`Actor.GetComponentByClass` _stationtarget "/Script/Engine.SceneComponent") _damage null)))))))

(fn `HitByBullet`
  (params (Damage :type Integer))
  (bind _hp (`self.Hp`))
  (bind _isdestroy (`self.IsDestroy`))
  (bind _output_get (set `self.CurrentHp` _hp))
  (bind _output_get_2 (set `self.Hp` (- _hp Damage)))
  (bind _asbp_main_game_mode (cast `/Game/BulletTrainAssets/Blueprints/BP_MainGameMode` (`GameplayStatics.GetGameMode`)))
  (if (not _isdestroy)
    (`/Game/BulletTrainAssets/Blueprints/BP_MainGameMode.GetScore` _asbp_main_game_mode (- _output_get _output_get_2))
    (if (<= _hp 0)
      (`/Engine/EditorBlueprintResources/StandardMacros.IsValid` (`self.GetOwner`)
        (:`Is Valid`
          (if (not _isdestroy)
            (`/Game/BulletTrainAssets/Blueprints/BP_MainGameMode.GetScore` _asbp_main_game_mode (`self.MaxHp`))
            (set `self.IsDestroy` true)))))))