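; BP_Weapon fires BP_Bullet projectiles from in front of its owner, tuned by WeaponData and the game mode's weapon settings.
; A looping timer advances the fire-rate counter, which gates Shoot and resets to a random offset to vary cadence.
; Each shot passes speed and damage to the bullet, adds heat to CharacterWeapon, flagging overheat when full, and plays sound, muzzle flash and camera shake.
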(event `self.ReceiveBeginPlay`
  (bind _asbp_main_game_mode (cast `/Game/BulletTrainAssets/Blueprints/BP_MainGameMode` (`GameplayStatics.GetGameMode`)))
  (bind _output_get (set `self.GameMode` _asbp_main_game_mode))
  (`KismetSystemLibrary.K2_SetTimer` null "Timer" (`/Game/BulletTrainAssets/Blueprints/BP_MainGameMode.TimerIntervalBase` _output_get) true))

(fn `Shoot`
  (bind _returnvalue (`self.GetOwner`))
  (bind _characterweapon (`self.CharacterWeapon`))
  (bind (_actor _camshakebase _firesound _name _damage _size _speed _nextreloadrange _heatpercent _firerate _bulletspawnposmul _bulletscale) (break `/Game/BulletTrainAssets/Blueprints/Structure/Weapon/WeaponData` (`self.WeaponData`)))
  (bind (_bulletsizebase _muzzleflashsizebase) (break `/Game/BulletTrainAssets/Blueprints/Structure/Weapon/WeaponSetting` (`/Game/BulletTrainAssets/Blueprints/BP_MainGameMode.WeaponSetting` (`self.GameMode`))))
  (bind _returnvalue_2 (+ (* (`Actor.GetActorForwardVector` _returnvalue) _bulletspawnposmul) (`Actor.K2_GetActorLocation` _returnvalue)))
  ;[0.05 0.05 0.05] Projectile Spawn Logic
  (if (>= (`self.FireRateTimer`) _firerate)
    (bind _returnvalue_3 (`|SpawnActorFromClass` "/Game/BulletTrainAssets/Blueprints/Weapon/BP_Bullet.BP_Bullet_C" (`KismetMathLibrary.MakeTransform` _returnvalue_2 (.rotation (`Actor.GetTransform` _returnvalue)) (* _bulletsizebase _bulletscale)) "Undefined" "OverrideRootScale" null null))
    (`/Engine/EditorBlueprintResources/StandardMacros.IsValid` _returnvalue_3
      (:`Is Valid`
        (set `/Game/BulletTrainAssets/Blueprints/Weapon/BP_Bullet.Speed` _speed _returnvalue_3)
        (set `/Game/BulletTrainAssets/Blueprints/Weapon/BP_Bullet.Damage` _damage _returnvalue_3)
        (bind _output_get (set `/Game/BulletTrainAssets/Blueprints/Character/BP_CharacterWeapon.OverheatPercent` (+ (`/Game/BulletTrainAssets/Blueprints/Character/BP_CharacterWeapon.OverheatPercent` _characterweapon) _heatpercent) _characterweapon))
        (if (>= _output_get 1.0)
          (set `/Game/BulletTrainAssets/Blueprints/Character/BP_CharacterWeapon.IsOverheat` true _characterweapon))
        (set `self.FireRateTimer` (`KismetMathLibrary.RandomFloatInRange` (* _nextreloadrange -1.0) _nextreloadrange))
        (`GameplayStatics.PlaySoundAtLocation` _firesound _returnvalue_2 (struct) 0.5 1.0 0.0 null null null null) ; Play firing sound
        (`GameplayStatics.SpawnEmitterAtLocation` "/Game/BulletTrainAssets/Particles/P_MuzzlFlash.P_MuzzlFlash" _returnvalue_2 (struct) (* _bulletscale _muzzleflashsizebase))
        (`GameplayStatics.PlayWorldCameraShake` _camshakebase (`Actor.K2_GetActorLocation` (`self.GetOwner`)) 0.0 1000.0)))))

(fn `Timer`
  (if (<= (`self.FireRateTimer`) (`.FireRate_7_2DCACF304611D0F90050788ADB95CB39` (break `/Game/BulletTrainAssets/Blueprints/Structure/Weapon/WeaponData` (`self.WeaponData`))))
    (set `self.FireRateTimer` (+ (`self.FireRateTimer`) (`/Game/BulletTrainAssets/Blueprints/BP_MainGameMode.TimerIntervalBase` (`self.GameMode`))))))