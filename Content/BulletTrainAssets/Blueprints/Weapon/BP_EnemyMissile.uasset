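; BP_EnemyMissile is an enemy homing missile projectile that damages actors tagged "Alience".
; On BeginPlay it passes its HomingTargetComponent variable to ProjectileMovement as the homing target.
; When CollisionComponent overlaps a tagged actor, it calls HitByBullet on that actor's Aliance component with Damage, spawns a scaled-up explosion effect and sound, then destroys itself.
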(event `self.ReceiveBeginPlay`
  (bind _output_get (set `ProjectileMovementComponent.HomingTargetComponent` (`self.HomingTargetComponent`) (`self.ProjectileMovement`))))

(event `self.CollisionComponent.OnComponentBeginOverlap`
  (params (OverlappedComponent :type "PrimitiveComponent Object Reference") (OtherActor :type "Actor Object Reference") (OtherComp :type "PrimitiveComponent Object Reference") (OtherBodyIndex :type Integer) (bFromSweep :type Boolean) (SweepResult :type "HitResult Structure (by ref)"))
  (bind _returnvalue (`self.K2_GetActorLocation`))
  (if (`self.ActorHasTag` OtherActor "Alience")
    (`/Game/BulletTrainAssets/Blueprints/Alliance/Aliance.HitByBullet` (`self.GetComponentByClass` OtherActor "/Game/BulletTrainAssets/Blueprints/Alliance/Aliance.Aliance_C") (`KismetMathLibrary.Conv_IntToDouble` (`self.Damage`)))
    (`GameplayStatics.SpawnEmitterAtLocation` "/Game/BulletTrainAssets/Particles/P_Explosion.P_Explosion" _returnvalue (struct) (5.0 5.0 5.0))
    (`GameplayStatics.PlaySoundAtLocation` "/Game/BulletTrainAssets/Sound/Explosion3.Explosion3" _returnvalue (struct) 1.0 1.0 0.0 null null null null)
    (`self.K2_DestroyActor`) ; Then destroy this projectile
  ))

(fn `UserConstructionScript`)