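; BP_Weapon is a data-driven weapon that fires BP_PlayerBullet projectiles from just ahead of its owner, with sound, muzzle flash and camera shake.
; Shoot is gated by a fire-rate counter advanced by a looping timer at the GameDataManager's base interval.
; Each shot adds heat to CharacterWeapon, flagging overheat at full, and resets the counter to a random offset to vary the cadence.
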(event `self.ReceiveBeginPlay`
  (bind _asbp_game_data_manager (cast `/Game/BulletTrainAssets/Blueprints/Manager/BP_GameDataManager` (`GameplayStatics.GetGameInstance`)))
  (bind _output_get (set `self.GameDataManager` _asbp_game_data_manager))
  (`KismetSystemLibrary.K2_SetTimer` null "Timer" (`/Game/BulletTrainAssets/Blueprints/Manager/BP_GameDataManager.TimerIntervalBase` _output_get) true))

(fn `Shoot`
  (bind _returnvalue (`self.GetOwner`))
  (bind _characterweapon (`self.CharacterWeapon`))
  (bind (_actor _camshakebase _firesound _name _damage _size _speed _nextrandomreloadrange _heatpercent _firerate _bulletspawnposmul _bulletscale) (break `/Game/BulletTrainAssets/Blueprints/Structure/Weapon/WeaponData` (`self.WeaponData`)))
  (bind (_bulletsizebase _muzzleflashsizebase) (break `/Game/BulletTrainAssets/Blueprints/Structure/Weapon/WeaponSettingData` (`/Game/BulletTrainAssets/Blueprints/Manager/BP_GameDataManager.WeaponSettingData` (`self.GameDataManager`))))
  (bind _returnvalue_2 (+ (* (`Actor.GetActorForwardVector` _returnvalue) _bulletspawnposmul) (`Actor.K2_GetActorLocation` _returnvalue)))
  ;[0.05 0.05 0.05] Projectile Spawn Logic
  (if (>= (`self.FireRateTimer`) _firerate)
    (bind _returnvalue_3 (`|SpawnActorFromClass` "/Game/BulletTrainAssets/Blueprints/Weapon/BP_PlayerBullet.BP_PlayerBullet_C" (`KismetMathLibrary.MakeTransform` _returnvalue_2 (.rotation (`Actor.GetTransform` _returnvalue)) (* _bulletsizebase _bulletscale)) "Undefined" "OverrideRootScale" null _speed _damage null))
    (`/Engine/EditorBlueprintResources/StandardMacros.IsValid` _returnvalue_3
      (:`Is Valid`
        (bind _output_get (set `/Game/BulletTrainAssets/Blueprints/Character/BP_CharacterWeapon.OverheatPercent` (+ (`/Game/BulletTrainAssets/Blueprints/Character/BP_CharacterWeapon.OverheatPercent` _characterweapon) _heatpercent) _characterweapon))
        (if (>= _output_get 1.0)
          (set `/Game/BulletTrainAssets/Blueprints/Character/BP_CharacterWeapon.IsOverheat` true _characterweapon))
        (set `self.FireRateTimer` (`KismetMathLibrary.RandomFloatInRange` (* _nextrandomreloadrange -1.0) _nextrandomreloadrange))
        (`GameplayStatics.PlaySoundAtLocation` _firesound _returnvalue_2 (struct) (`/Game/BulletTrainAssets/Blueprints/Manager/BP_GameDataManager.EffectSoundVolum` (`self.GameDataManager`)) 1.0 0.0 null null null null) ; Play firing sound
        (`GameplayStatics.SpawnEmitterAtLocation` "/Game/BulletTrainAssets/Particles/P_MuzzlFlash.P_MuzzlFlash" _returnvalue_2 (struct) (* _bulletscale _muzzleflashsizebase))
        (`GameplayStatics.PlayWorldCameraShake` _camshakebase (`Actor.K2_GetActorLocation` (`self.GetOwner`)) 0.0 1000.0)))))

(fn `Timer`
  (if (<= (`self.FireRateTimer`) (`.FireRate_7_2DCACF304611D0F90050788ADB95CB39` (break `/Game/BulletTrainAssets/Blueprints/Structure/Weapon/WeaponData` (`self.WeaponData`))))
    (set `self.FireRateTimer` (+ (`self.FireRateTimer`) (`/Game/BulletTrainAssets/Blueprints/Manager/BP_GameDataManager.TimerIntervalBase` (`self.GameDataManager`))))))