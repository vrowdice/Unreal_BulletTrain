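; BP_EnemyMissile is an enemy homing missile projectile that damages actors tagged "Alience".
; On BeginPlay it assigns its HomingTargetComponent to the projectile movement and sets that target component to absolute rotation.
; On collision overlap with a tagged actor, it calls HitByBullet on the actor's Aliance component, then spawns a scaled-up explosion.
; The explosion sound uses the GameDataManager game instance's effect volume, and the missile then destroys itself.
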(event `self.ReceiveBeginPlay`
  (bind _output_get (set `ProjectileMovementComponent.HomingTargetComponent` (`self.HomingTargetComponent`) (`self.ProjectileMovement`)))
  (set `SceneComponent.bAbsoluteRotation` true _output_get))

(event `self.CollisionComponent.OnComponentBeginOverlap`
  (params (OverlappedComponent :type "PrimitiveComponent Object Reference") (OtherActor :type "Actor Object Reference") (OtherComp :type "PrimitiveComponent Object Reference") (OtherBodyIndex :type Integer) (bFromSweep :type Boolean) (SweepResult :type "HitResult Structure (by ref)"))
  (bind _returnvalue (`self.K2_GetActorLocation`))
  (if (`self.ActorHasTag` OtherActor "Alience")
    (`/Game/BulletTrainAssets/Blueprints/Alliance/Aliance.HitByBullet` (`self.GetComponentByClass` OtherActor "/Game/BulletTrainAssets/Blueprints/Alliance/Aliance.Aliance_C") (`KismetMathLibrary.Conv_IntToDouble` (`self.Damage`)))
    (bind _asbp_game_data_manager (cast `/Game/BulletTrainAssets/Blueprints/Manager/BP_GameDataManager` (`GameplayStatics.GetGameInstance`)))
    (`GameplayStatics.SpawnEmitterAtLocation` "/Game/BulletTrainAssets/Particles/P_Explosion.P_Explosion" _returnvalue (struct) (5.0 5.0 5.0))
    (`GameplayStatics.PlaySoundAtLocation` "/Game/BulletTrainAssets/Sound/Explosion/Explosion3.Explosion3" _returnvalue (struct) (`/Game/BulletTrainAssets/Blueprints/Manager/BP_GameDataManager.EffectSoundVolum` _asbp_game_data_manager) 1.0 0.0 null null null null)
    (`self.K2_DestroyActor`) ; Then destroy this projectile
  ))

(fn `UserConstructionScript`)