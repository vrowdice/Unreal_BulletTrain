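; BP_EnemyBullet is a projectile fired by enemies that flies toward a given ShootTarget and damages allied actors.
; On BeginPlay it rotates to face the target's location and sets the ProjectileMovement velocity along Sphere1's forward vector, with no later steering in the graph.
; When its collision component overlaps an actor tagged "Alience", it calls HitByBullet on that actor's Aliance component, spawns an explosion particle and destroys itself.
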(event `self.ReceiveBeginPlay`
  (`self.K2_SetActorRotation` (`KismetMathLibrary.FindLookAtRotation` (`self.K2_GetActorLocation`) (`self.K2_GetActorLocation` (`self.ShootTarget`))))
  (set `MovementComponent.Velocity` (* (`SceneComponent.GetForwardVector` (`self.Sphere1`)) (`ProjectileMovementComponent.InitialSpeed` (`self.ProjectileMovement`))) (`self.ProjectileMovement`)))

(event `self.CollisionComponent.OnComponentBeginOverlap`
  (params (OverlappedComponent :type "PrimitiveComponent Object Reference") (OtherActor :type "Actor Object Reference") (OtherComp :type "PrimitiveComponent Object Reference") (OtherBodyIndex :type Integer) (bFromSweep :type Boolean) (SweepResult :type "HitResult Structure (by ref)"))
  (if (`self.ActorHasTag` OtherActor "Alience")
    (`/Game/BulletTrainAssets/Blueprints/Alliance/Aliance.HitByBullet` (`self.GetComponentByClass` OtherActor "/Game/BulletTrainAssets/Blueprints/Alliance/Aliance.Aliance_C") (`KismetMathLibrary.Conv_IntToDouble` (`self.Damage`)))
    (`GameplayStatics.SpawnEmitterAtLocation` "/Game/BulletTrainAssets/Particles/P_Explosion.P_Explosion" (`self.K2_GetActorLocation`))
    (`self.K2_DestroyActor`) ; Then destroy this projectile
  ))

(fn `UserConstructionScript`)